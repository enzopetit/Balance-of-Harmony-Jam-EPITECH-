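; Master AI enemy character that spots the FPS player, carries a rifle, takes damage and dies.
; BeginPlay sets health, links its UI widget and spawns the rifle onto the back socket.
; Seeing the player or taking body damage sets PlayerFound; combat entry plays an equip montage, while a separate FlipFlop event swaps the rifle between back and hand.
; Headshots kill instantly, and death ragdolls the mesh before destroying pawn and weapon after a delay.
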(event OnSeePawn(PawnSensing)
  (params (Pawn :type Pawn%20Object%20Reference))
  (Utilities|Casting|CastToFPS_Character Pawn)
  (Variables|Default|SetPlayerFound? true))

(event Custom|Equip/Unequip
  (Utilities|FlowControl|FlipFlop
    (:A
      (Transformation|AttachComponentToComponent (Variables|Default|GetAIWeaponRef) (Variables|Character|GetMesh) "WeaponHold" "KeepRelative" "KeepRelative" "KeepRelative" true)
      (Variables|Default|SetEquipWeapon true))
    (:B
      (Transformation|AttachComponentToComponent (Variables|Default|GetAIWeaponRef) (Variables|Character|GetMesh) "WeaponBack" "KeepRelative" "KeepRelative" "KeepRelative" true)
      (Variables|Default|SetEquipWeapon false))))

(event Custom|SpawnWeapon
  (bind _returnvalue (Game|SpawnActorfromClass "/Game/Core/AI/BPC_AI_Rifle.BPC_AI_Rifle_C" (Transformation|GetWorldTransform (Variables|Default|GetWeaponSpawn)) "Undefined" 0 0))
  (bind _output_get (Variables|Default|SetAIWeaponRef _returnvalue))
  (Transformation|AttachComponentToComponent _output_get (Variables|Character|GetMesh) "WeaponBack" "KeepWorld" "KeepWorld" "KeepWorld" true))

(event Custom|EnterCombatMode
  (Animation|Montage|PlayMontage (Variables|Character|GetMesh) "/Game/Core/AI/Animations/AM_EquipWeapon.AM_EquipWeapon"
    (:OnCompleted
      (Variables|Default|SetAnimDone? true))))

(event EventBeginPlay
  (Variables|Default|SetCurrentHealth (Variables|Default|GetMaxHealth))
  (bind _asui_ai (Utilities|Casting|CastToUI_AI (UserInterface|GetUserWidgetObject (Variables|Default|GetWidget))))
  (Variables|/Game/Core/AI/UI_AI.UI_AI_C|SetOwner _asui_ai self)
  (CallFunction|SpawnWeapon))

(event EventTakeDamage
  (params (BoneName :type Name :default "None") (Damage :type Float%20%28single-precision%29))
  (bind _mesh (Variables|Character|GetMesh))
  (if (Utilities|Name|Equal(Name) BoneName "Head")
    (Variables|Default|SetCurrentHealth 0.0)
    (else
      (Variables|Default|SetPlayerFound? true)
      (Variables|Default|SetCurrentHealth (- (Variables|Default|GetCurrentHealth) Damage))))
  (if (<= (Variables|Default|GetCurrentHealth) 0.0)
    (Variables|Default|SetAIDead? true)
    (Class|SkeletalMeshComponent|SetAllBodiesSimulatePhysics _mesh true)
    (Collision|SetCollisionEnabled _mesh "QueryAndPhysics")
    (Collision|SetCollisionEnabled (Variables|Collision|GetCapsuleComponent) "NoCollision")
    (Utilities|FlowControl|Delay 5.0)
    (Actor|DestroyActor (Variables|Default|GetAIWeaponRef))
    (Actor|DestroyActor)))

(fn ConstructionScript)