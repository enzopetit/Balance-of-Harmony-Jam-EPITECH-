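; BP_ItemMaster is a pickup item, handling Armor and Health Pack types through an ItemType switch.
; Trigger overlap with FPS_Character toggles a custom-depth highlight, a prompt widget and CanBePicked, and enables player input on entry.
; Interagir refills armor to MaxArmor or increments the HealthPack count, then destroys the actor.
; Armor pickup is refused at a hardcoded 100 threshold, clearing CanBePicked and printing a message.
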(event OnComponentBeginOverlap(Trigger)
  (params (OverlappedComponent :type Primitive%20Component%20Object%20Reference) (OtherActor :type Actor%20Object%20Reference) (OtherComp :type Primitive%20Component%20Object%20Reference) (OtherBodyIndex :type Integer) (bFromSweep :type Boolean) (SweepResult :type Hit%20Result%20Structure%20%28by%20ref%29))
  (Utilities|Casting|CastToFPS_Character OtherActor)
  (Rendering|SetRenderCustomDepth (Variables|Default|GetSM_Item) true)
  (Rendering|SetVisibility (Variables|Default|GetWidget) true false)
  (Variables|Default|SetCanBePicked? true)
  (Input|EnableInput (Game|GetPlayerController 0)))

(event OnComponentEndOverlap(Trigger)
  (params (OverlappedComponent :type Primitive%20Component%20Object%20Reference) (OtherActor :type Actor%20Object%20Reference) (OtherComp :type Primitive%20Component%20Object%20Reference) (OtherBodyIndex :type Integer))
  (Utilities|Casting|CastToFPS_Character OtherActor)
  (Rendering|SetRenderCustomDepth (Variables|Default|GetSM_Item) false)
  (Rendering|SetVisibility (Variables|Default|GetWidget) false false)
  (Variables|Default|SetCanBePicked? false))

(event Input|ActionEvents|InputActionInteragir
  (params (Key :type Key%20Structure :default "None"))
  (bind _returnvalue (Game|GetPlayerCharacter 0))
  (:Pressed
    (if (Variables|Default|GetCanBePicked?)
      (switch Utilities|FlowControl|Switch|SwitchonE_ItemType (Variables|Default|GetItemType)
        (:NewEnumerator1
          (bind _asfps_character (Utilities|Casting|CastToFPS_Character _returnvalue))
          (if (>= (Variables|/Game/Core/PlayerCharacter/FPS_Character.FPS_Character_C|GetCurrentArmor _asfps_character) 1e+02)
            (Variables|Default|SetCanBePicked? false)
            (Development|PrintString "Tu peux pas recup")
            (else
              (Variables|/Game/Core/PlayerCharacter/FPS_Character.FPS_Character_C|SetCurrentArmor _asfps_character (Variables|/Game/Core/PlayerCharacter/FPS_Character.FPS_Character_C|GetMaxArmor _asfps_character))
              (Actor|DestroyActor))))
        (:NewEnumerator2
          (bind _asfps_character_2 (Utilities|Casting|CastToFPS_Character _returnvalue))
          (bind _result (Math|Integer|IncrementInt (Variables|/Game/Core/PlayerCharacter/FPS_Character.FPS_Character_C|GetHealthPack _asfps_character_2))
            (:%20%20
              (Variables|/Game/Core/PlayerCharacter/FPS_Character.FPS_Character_C|SetHealthPack _asfps_character_2 _result)
              (Actor|DestroyActor))))))))

(fn ConstructionScript)