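; BP_Bullets is a bullet projectile actor that reacts to hits and then destroys itself.
; On every hit it fires its RadialForce impulse.
; Physics-simulating components also get an impulse at the bullet's location, scaled from its velocity by BulletImpulse, unless the hit actor is a BP_AIMaster or FPS_Character.
; The graph applies no damage.
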(event Collision|EventHit
  (params (MyComp :type Primitive%20Component%20Object%20Reference) (Other :type Actor%20Object%20Reference) (OtherComp :type Primitive%20Component%20Object%20Reference) (bSelfMoved :type Boolean) (HitLocation :type Vector :default "0, 0, 0") (HitNormal :type Vector :default "0, 0, 0") (NormalImpulse :type Vector :default "0, 0, 0") (Hit :type Hit%20Result%20Structure%20%28by%20ref%29))
  (Class|RadialForceComponent|FireImpulse (Variables|Default|GetRadialForce))
  (if (Physics|IsSimulatingPhysics OtherComp "None")
    (if (or (Utilities|IsValid (.AsBP%20AIMaster (Utilities|Casting|CastToBP_AIMaster Other))) (Utilities|IsValid (.AsFPS%20Character (Utilities|Casting|CastToFPS_Character Other))))
      (Actor|DestroyActor :!label _label)
      (else
        (Physics|AddImpulseatLocation OtherComp (* (Transformation|GetVelocity) (Variables|Default|GetBulletImpulse)) (Transformation|GetActorLocation) "None")
        (Actor|DestroyActor)))
    (else
      (goto _label))))

(fn ConstructionScript)